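; Practice shelf puzzle where an alarm clock, duck, rocket and robot must each reach their colored pedestal before time runs out.
; Sphere overlaps glow red for wrong objects; correct ones are released from the hand, attached, locked, turned gold and lit green.
; Tick drives a Delay-based countdown, toggling the alarm light below a minute.
; Completion or timeout opens the door and shows exit signs; success turns the alarm light green.
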(event `self.ReceiveBeginPlay`
  (`self.Set Spheres`))

(event `self.ReceiveTick`
  (params (DeltaSeconds :type "Float (single-precision)"))
  (if (== (`self.Seconds`) 0)
    (`self.TimeOut`)
    (elif (and (`self.OverlapObject01`) (`self.OverlapObject02`) (`self.OverlapObject03`) (`self.OverlapObject04`))
      (`self.FinishedRoom`)
      (else
        (`KismetSystemLibrary.Delay` 1.0)
        (set `self.Seconds` (- (`self.Seconds`) 1))
        (if (< (`self.Seconds`) 60)
          (`SceneComponent.ToggleVisibility` (`/Game/SpatialImmersion/Blueprint/Gamification/BP_Alarmlight.SpotLight` (`self.Alarmlight`)) false))))))

(event `self.Sphere_Pedestal_Red.OnComponentBeginOverlap`
  (params (OverlappedComponent :type "PrimitiveComponent Object Reference") (OtherActor :type "Actor Object Reference") (OtherComp :type "PrimitiveComponent Object Reference") (OtherBodyIndex :type Integer) (bFromSweep :type Boolean) (SweepResult :type "HitResult Structure (by ref)"))
  (if (`self.IsOverlappingActor` OtherActor (`self.Alarmclock`))
    (`self.Attach Object 01` OtherActor)
    (else
      (`PrimitiveComponent.SetMaterial` (`self.Light_Pedestal_Red`) 0 "/Game/SpatialImmersion/Material/GlowingMaterial/MI_Pulsing_Glow_Red.MI_Pulsing_Glow_Red"))))

(event `self.Sphere_Pedestal_Red.OnComponentEndOverlap`
  (params (OverlappedComponent :type "PrimitiveComponent Object Reference") (OtherActor :type "Actor Object Reference") (OtherComp :type "PrimitiveComponent Object Reference") (OtherBodyIndex :type Integer))
  (bind _light_pedestal_red (`self.Light_Pedestal_Red`))
  (if (`self.OverlapObject01`)
    (`PrimitiveComponent.SetMaterial` _light_pedestal_red 0 "/Game/SpatialImmersion/Material/GlowingMaterial/MI_Pulsing_Glow_Green.MI_Pulsing_Glow_Green")
    (else
      (`PrimitiveComponent.SetMaterial` _light_pedestal_red 0 "/Game/SpatialImmersion/Material/Colours/Luminous_Colour/_Glowing_Lamp_Pedestal._Glowing_Lamp_Pedestal"))))

(event `self.Sphere_Pedestal_Blue.OnComponentBeginOverlap`
  (params (OverlappedComponent :type "PrimitiveComponent Object Reference") (OtherActor :type "Actor Object Reference") (OtherComp :type "PrimitiveComponent Object Reference") (OtherBodyIndex :type Integer) (bFromSweep :type Boolean) (SweepResult :type "HitResult Structure (by ref)"))
  (if (`self.IsOverlappingActor` OtherActor (`self.Duck`))
    (`self.Attach Object 02` OtherActor)
    (else
      (`PrimitiveComponent.SetMaterial` (`self.Light_Pedestal_Blue`) 0 "/Game/SpatialImmersion/Material/GlowingMaterial/MI_Pulsing_Glow_Red.MI_Pulsing_Glow_Red"))))

(event `self.Sphere_Pedestal_Blue.OnComponentEndOverlap`
  (params (OverlappedComponent :type "PrimitiveComponent Object Reference") (OtherActor :type "Actor Object Reference") (OtherComp :type "PrimitiveComponent Object Reference") (OtherBodyIndex :type Integer))
  (bind _light_pedestal_blue (`self.Light_Pedestal_Blue`))
  (if (`self.OverlapObject02`)
    (`PrimitiveComponent.SetMaterial` _light_pedestal_blue 0 "/Game/SpatialImmersion/Material/GlowingMaterial/MI_Pulsing_Glow_Green.MI_Pulsing_Glow_Green")
    (else
      (`PrimitiveComponent.SetMaterial` _light_pedestal_blue 0 "/Game/SpatialImmersion/Material/Colours/Luminous_Colour/_Glowing_Lamp_Pedestal._Glowing_Lamp_Pedestal"))))

(event `self.Sphere_Pedestal_Green.OnComponentBeginOverlap`
  (params (OverlappedComponent :type "PrimitiveComponent Object Reference") (OtherActor :type "Actor Object Reference") (OtherComp :type "PrimitiveComponent Object Reference") (OtherBodyIndex :type Integer) (bFromSweep :type Boolean) (SweepResult :type "HitResult Structure (by ref)"))
  (if (`self.IsOverlappingActor` OtherActor (`self.Rocket`))
    (`self.Attach Object 03` OtherActor)
    (else
      (`PrimitiveComponent.SetMaterial` (`self.Light_Pedestal_Green`) 0 "/Game/SpatialImmersion/Material/GlowingMaterial/MI_Pulsing_Glow_Red.MI_Pulsing_Glow_Red"))))

(event `self.Sphere_Pedestal_Green.OnComponentEndOverlap`
  (params (OverlappedComponent :type "PrimitiveComponent Object Reference") (OtherActor :type "Actor Object Reference") (OtherComp :type "PrimitiveComponent Object Reference") (OtherBodyIndex :type Integer))
  (bind _light_pedestal_green (`self.Light_Pedestal_Green`))
  (if (`self.OverlapObject03`)
    (`PrimitiveComponent.SetMaterial` _light_pedestal_green 0 "/Game/SpatialImmersion/Material/GlowingMaterial/MI_Pulsing_Glow_Green.MI_Pulsing_Glow_Green")
    (else
      (`PrimitiveComponent.SetMaterial` _light_pedestal_green 0 "/Game/SpatialImmersion/Material/Colours/Luminous_Colour/_Glowing_Lamp_Pedestal._Glowing_Lamp_Pedestal"))))

(event `self.Sphere_Pedestal_Orange.OnComponentBeginOverlap`
  (params (OverlappedComponent :type "PrimitiveComponent Object Reference") (OtherActor :type "Actor Object Reference") (OtherComp :type "PrimitiveComponent Object Reference") (OtherBodyIndex :type Integer) (bFromSweep :type Boolean) (SweepResult :type "HitResult Structure (by ref)"))
  (if (`self.IsOverlappingActor` OtherActor (`self.Robot`))
    (`self.Attach Object 04` OtherActor)
    (else
      (`PrimitiveComponent.SetMaterial` (`self.Light_Pedestal_Orange`) 0 "/Game/SpatialImmersion/Material/GlowingMaterial/MI_Pulsing_Glow_Red.MI_Pulsing_Glow_Red"))))

(event `self.Sphere_Pedestal_Orange.OnComponentEndOverlap`
  (params (OverlappedComponent :type "PrimitiveComponent Object Reference") (OtherActor :type "Actor Object Reference") (OtherComp :type "PrimitiveComponent Object Reference") (OtherBodyIndex :type Integer))
  (bind _light_pedestal_orange (`self.Light_Pedestal_Orange`))
  (if (`self.OverlapObject04`)
    (`PrimitiveComponent.SetMaterial` _light_pedestal_orange 0 "/Game/SpatialImmersion/Material/GlowingMaterial/MI_Pulsing_Glow_Green.MI_Pulsing_Glow_Green")
    (else
      (`PrimitiveComponent.SetMaterial` _light_pedestal_orange 0 "/Game/SpatialImmersion/Material/Colours/Luminous_Colour/_Glowing_Lamp_Pedestal._Glowing_Lamp_Pedestal"))))

(fn `Attach Object 01`
  (params (Object :type "Object Object Reference"))
  (bind _sphere_red (`self.Sphere_Red`))
  (bind _asbp_pa_alarmclock (cast `/Game/SpatialImmersion/Blueprint/Stylized/BP_PA_Alarmclock` Object))
  (set `self.OverlapObject01` true)
  (`self.K2_DetachFromActor` _asbp_pa_alarmclock "KeepWorld" "KeepWorld" "KeepWorld")
  (`PickupActor.ReleaseFromHand` _asbp_pa_alarmclock)
  (`PrimitiveComponent.SetSimulatePhysics` (`PickupActor.StaticMeshComponent` _asbp_pa_alarmclock) false)
  (`self.K2_SetActorLocation` _asbp_pa_alarmclock (`SceneComponent.K2_GetComponentLocation` (`self.Sphere_Pedestal_Red`)) false false)
  (`self.K2_AttachToComponent` _asbp_pa_alarmclock (`self.Pedestal_Red`) "None" "SnapToTarget" "KeepRelative" "KeepRelative" true)
  (set `PickupActor.bIsActiveForInteraction` false _asbp_pa_alarmclock)
  (bind _staticmeshcomponent (`PickupActor.StaticMeshComponent` _asbp_pa_alarmclock))
  (`PrimitiveComponent.SetMaterialByName` _staticmeshcomponent "MI_Clock" "/Game/SpatialImmersion/Material/Gold/MI_Gold.MI_Gold")
  (`SceneComponent.K2_SetWorldRotation` _staticmeshcomponent (struct :`Yaw` 90.0) false false)
  (`PrimitiveComponent.SetMaterialByName` (`self.Pedestal_Red`) "Light" "/Game/SpatialImmersion/Material/ArchViz/MI_WoodVeneer2.MI_WoodVeneer2")
  (`self.K2_DestroyActor` (`self.Torus_Object01`))
  (`PrimitiveComponent.SetMaterial` (`self.Light_Pedestal_Red`) 0 "/Game/SpatialImmersion/Material/GlowingMaterial/MI_Pulsing_Glow_Green.MI_Pulsing_Glow_Green")
  (`SceneComponent.SetVisibility` _sphere_red true false)
  (`PrimitiveComponent.SetCollisionResponseToAllChannels` _sphere_red "ECR_Block"))

(fn `Attach Object 02`
  (params (Object :type "Object Object Reference"))
  (bind _sphere_blue (`self.Sphere_Blue`))
  (bind _asbp_pa_duck_02 (cast `/Game/SpatialImmersion/Blueprint/Stylized/BP_PA_Duck02` Object))
  (set `self.OverlapObject02` true)
  (`self.K2_DetachFromActor` _asbp_pa_duck_02 "KeepWorld" "KeepWorld" "KeepWorld")
  (`PickupActor.ReleaseFromHand` _asbp_pa_duck_02)
  (`PrimitiveComponent.SetSimulatePhysics` (`PickupActor.StaticMeshComponent` _asbp_pa_duck_02) false)
  (`self.K2_SetActorLocation` _asbp_pa_duck_02 (`SceneComponent.K2_GetComponentLocation` (`self.Sphere_Pedestal_Blue`)) false false)
  (`self.K2_AttachToComponent` _asbp_pa_duck_02 (`self.Pedestal_Blue`) "None" "SnapToTarget" "KeepWorld" "KeepRelative" true)
  (set `PickupActor.bIsActiveForInteraction` false _asbp_pa_duck_02)
  (bind _staticmeshcomponent (`PickupActor.StaticMeshComponent` _asbp_pa_duck_02))
  (`SceneComponent.K2_SetWorldRotation` _staticmeshcomponent (struct :`Yaw` 90.0) false false)
  (for _array_element (`MeshComponent.GetMaterialSlotNames` _staticmeshcomponent)
    (`PrimitiveComponent.SetMaterialByName` _staticmeshcomponent _array_element "/Game/SpatialImmersion/Material/Gold/MI_Gold.MI_Gold"))
  (`PrimitiveComponent.SetMaterialByName` (`self.Pedestal_Blue`) "Light" "/Game/SpatialImmersion/Material/ArchViz/MI_WoodVeneer2.MI_WoodVeneer2")
  (`self.K2_DestroyActor` (`self.Torus_Object02`))
  (`SceneComponent.SetVisibility` _sphere_blue true false)
  (`PrimitiveComponent.SetCollisionResponseToAllChannels` _sphere_blue "ECR_Block")
  (`PrimitiveComponent.SetMaterial` (`self.Light_Pedestal_Blue`) 0 "/Game/SpatialImmersion/Material/GlowingMaterial/MI_Pulsing_Glow_Green.MI_Pulsing_Glow_Green"))

(fn `Attach Object 03`
  (params (Object :type "Object Object Reference"))
  (bind _sphere_green (`self.Sphere_Green`))
  (bind _asbp_pa_rocket_umg (cast `/Game/SpatialImmersion/Blueprint/Stylized/BP_PA_Rocket_UMG` Object))
  (set `self.OverlapObject03` true)
  (`self.K2_DetachFromActor` _asbp_pa_rocket_umg "KeepWorld" "KeepWorld" "KeepWorld")
  (`PickupActor.ReleaseFromHand` _asbp_pa_rocket_umg)
  (`PrimitiveComponent.SetSimulatePhysics` (`PickupActor.StaticMeshComponent` _asbp_pa_rocket_umg) false)
  (`self.K2_SetActorLocation` _asbp_pa_rocket_umg (`SceneComponent.K2_GetComponentLocation` (`self.Sphere_Pedestal_Green`)) false false)
  (`self.K2_AttachToComponent` _asbp_pa_rocket_umg (`self.Pedestal_Green`) "None" "SnapToTarget" "KeepWorld" "KeepRelative" true)
  (set `PickupActor.bIsActiveForInteraction` false _asbp_pa_rocket_umg)
  (bind _staticmeshcomponent (`PickupActor.StaticMeshComponent` _asbp_pa_rocket_umg))
  (`SceneComponent.K2_SetWorldRotation` _staticmeshcomponent (struct :`Yaw` 90.0) false false)
  (for _array_element (`MeshComponent.GetMaterialSlotNames` _staticmeshcomponent)
    (`PrimitiveComponent.SetMaterialByName` _staticmeshcomponent _array_element "/Game/SpatialImmersion/Material/Gold/MI_Gold.MI_Gold"))
  (`PrimitiveComponent.SetMaterialByName` (`self.Pedestal_Green`) "Light" "/Game/SpatialImmersion/Material/ArchViz/MI_WoodVeneer2.MI_WoodVeneer2")
  (`self.SetActorScale3D` _asbp_pa_rocket_umg (0.5 0.5 0.5))
  (`self.K2_DestroyActor` (`self.Torus_Object03`))
  (`SceneComponent.SetVisibility` _sphere_green true false)
  (`PrimitiveComponent.SetCollisionResponseToAllChannels` _sphere_green "ECR_Block")
  (`PrimitiveComponent.SetMaterial` (`self.Light_Pedestal_Green`) 0 "/Game/SpatialImmersion/Material/GlowingMaterial/MI_Pulsing_Glow_Green.MI_Pulsing_Glow_Green"))

(fn `Attach Object 04`
  (params (Object :type "Object Object Reference"))
  (bind _sphere_orange (`self.Sphere_Orange`))
  (bind _asbp_pa_robot_umg (cast `/Game/SpatialImmersion/Blueprint/Stylized/BP_PA_Robot_UMG` Object))
  (set `self.OverlapObject04` true)
  (`self.K2_DetachFromActor` _asbp_pa_robot_umg "KeepWorld" "KeepWorld" "KeepWorld")
  (`PickupActor.ReleaseFromHand` _asbp_pa_robot_umg)
  (`PrimitiveComponent.SetSimulatePhysics` (`PickupActor.StaticMeshComponent` _asbp_pa_robot_umg) false)
  (`self.K2_SetActorLocation` _asbp_pa_robot_umg (`SceneComponent.K2_GetComponentLocation` (`self.Sphere_Pedestal_Orange`)) false false)
  (`self.K2_AttachToComponent` _asbp_pa_robot_umg (`self.Pedestal_Orange`) "None" "SnapToTarget" "KeepWorld" "KeepRelative" true)
  (set `PickupActor.bIsActiveForInteraction` false _asbp_pa_robot_umg)
  (bind _staticmeshcomponent (`PickupActor.StaticMeshComponent` _asbp_pa_robot_umg))
  (`SceneComponent.K2_SetWorldRotation` _staticmeshcomponent (struct :`Yaw` 90.0) false false)
  (`self.K2_DestroyActor` (`self.Torus_Object04`))
  (for _array_element (`MeshComponent.GetMaterialSlotNames` _staticmeshcomponent)
    (`PrimitiveComponent.SetMaterialByName` _staticmeshcomponent _array_element "/Game/SpatialImmersion/Material/Gold/MI_Gold.MI_Gold"))
  (`self.SetActorScale3D` _asbp_pa_robot_umg (0.5 0.5 0.5))
  (`PrimitiveComponent.SetMaterialByName` (`self.Pedestal_Orange`) "Light" "/Game/SpatialImmersion/Material/ArchViz/MI_WoodVeneer2.MI_WoodVeneer2")
  (`SceneComponent.SetVisibility` _sphere_orange true false)
  (`PrimitiveComponent.SetCollisionResponseToAllChannels` _sphere_orange "ECR_Block")
  (`PrimitiveComponent.SetMaterial` (`self.Light_Pedestal_Orange`) 0 "/Game/SpatialImmersion/Material/GlowingMaterial/MI_Pulsing_Glow_Green.MI_Pulsing_Glow_Green"))

(fn `FinishedRoom`
  (bind _spotlight (`/Game/SpatialImmersion/Blueprint/Gamification/BP_Alarmlight.SpotLight` (`self.Alarmlight`)))
  (bind _staticmesh (`/Game/SpatialImmersion/Blueprint/UMG/BP_Sign_Exit.StaticMesh` (`self.Sign`)))
  (`SceneComponent.SetVisibility` (`/Game/SpatialImmersion/Blueprint/Gamification/BP_Emergency_Exit_Sign.Plane` (`self.Exit sign`)) true false)
  (`SceneComponent.SetVisibility` (`/Game/SpatialImmersion/Blueprint/Gamification/BP_Emergency_Exit_Sign.StaticMesh` (`self.Exit sign`)) true false)
  (`SceneComponent.SetVisibility` _spotlight true false)
  (`LightComponent.SetLightColor` _spotlight (struct :`R` 0.01003 :`G` 0.354167 :`A` 1.0) true)
  (`SceneComponent.K2_SetWorldRotation` (`/Game/SpatialImmersion/Blueprint/BP_Door.Door` (`self.Door`)) (struct :`Yaw` 180.0) false false)
  (set `self.Level` true)
  (`SceneComponent.SetVisibility` _staticmesh true false)
  (`PrimitiveComponent.SetCollisionResponseToChannel` _staticmesh "ECC_WorldStatic" "ECR_Block")
  (`PrimitiveComponent.SetCollisionResponseToChannel` _staticmesh "ECC_WorldStatic" "ECR_Overlap"))

(fn `Set Spheres`
  (bind _sphere_blue (`self.Sphere_Blue`))
  (bind _sphere_green (`self.Sphere_Green`))
  (bind _sphere_orange (`self.Sphere_Orange`))
  (bind _sphere_red (`self.Sphere_Red`))
  (`SceneComponent.SetVisibility` _sphere_red false false)
  (`PrimitiveComponent.SetCollisionResponseToAllChannels` _sphere_red "ECR_Ignore")
  (`SceneComponent.SetVisibility` _sphere_blue false false)
  (`PrimitiveComponent.SetCollisionResponseToAllChannels` _sphere_blue "ECR_Ignore")
  (`SceneComponent.SetVisibility` _sphere_green false false)
  (`PrimitiveComponent.SetCollisionResponseToAllChannels` _sphere_green "ECR_Ignore")
  (`SceneComponent.SetVisibility` _sphere_orange false false)
  (`PrimitiveComponent.SetCollisionResponseToAllChannels` _sphere_orange "ECR_Ignore"))

(fn `TimeOut`
  (bind _staticmesh (`/Game/SpatialImmersion/Blueprint/UMG/BP_Sign_Exit.StaticMesh` (`self.Sign`)))
  (`SceneComponent.SetVisibility` (`/Game/SpatialImmersion/Blueprint/Gamification/BP_Alarmlight.SpotLight` (`self.Alarmlight`)) true false)
  (`SceneComponent.SetVisibility` (`/Game/SpatialImmersion/Blueprint/Gamification/BP_Emergency_Exit_Sign.Plane` (`self.Exit sign`)) true false)
  (`SceneComponent.SetVisibility` (`/Game/SpatialImmersion/Blueprint/Gamification/BP_Emergency_Exit_Sign.StaticMesh` (`self.Exit sign`)) true false)
  (`SceneComponent.K2_SetWorldRotation` (`/Game/SpatialImmersion/Blueprint/BP_Door.Door` (`self.Door`)) (struct :`Yaw` 180.0) false false)
  (set `self.Level` true)
  (`SceneComponent.SetVisibility` _staticmesh true false)
  (`PrimitiveComponent.SetCollisionResponseToChannel` _staticmesh "ECC_WorldStatic" "ECR_Block")
  (`PrimitiveComponent.SetCollisionResponseToChannel` _staticmesh "ECC_WorldStatic" "ECR_Overlap"))

(fn `UserConstructionScript`)