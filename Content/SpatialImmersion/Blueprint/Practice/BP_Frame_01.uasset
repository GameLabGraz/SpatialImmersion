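; BP_Frame_01 is a picture frame in the SpatialImmersion practice content whose image follows a Handle's rotation.
; Each tick it shows the Papyrus material when the Handle is turned past 60 degrees, otherwise the Gleaners material.
; The first time past that threshold, a one-shot Spawn flag reveals the new torus, arrow hint and decal, hides the old cues, and sets a New_Task widget on the Sign.
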(event `self.ReceiveTick`
  (params (DeltaSeconds :type "Float (single-precision)"))
  (if (> (`CircularDriveActor.CurrentRotation` (`self.Handle`)) 60.0)
    (`PrimitiveComponent.SetMaterial` (`self.StaticMesh`) 1 "/Game/SpatialImmersion/Material/Pattern/Museum/Pictures/Papyrus01_Mat.Papyrus01_Mat")
    (if (`self.Spawn`)
      (set `self.Spawn` false)
      (`SceneComponent.SetVisibility` (`/Game/SpatialImmersion/Blueprint/Practice/BP_Teleport_Torus_Slider.StaticMesh` (`self.Torus_New`)) true false)
      (`SceneComponent.SetVisibility` (`/Game/SpatialImmersion/Blueprint/Practice/BP_Teleport_Torus_Slider.Arrow` (`self.Torus_New`)) true false)
      (`SceneComponent.SetVisibility` (`/Game/SpatialImmersion/Blueprint/Gamification/BP_Arrow_Hint.StaticMesh` (`self.Arrow_Hint`)) true false)
      (`SceneComponent.SetVisibility` (`DecalActor.Decal` (`self.Decal`)) true false)
      (`SceneComponent.SetVisibility` (`/Game/SpatialImmersion/Blueprint/Practice/BP_Teleport_Torus_Handle.StaticMesh` (`self.Torus_Old`)) false false)
      (`SceneComponent.SetVisibility` (`/Game/SpatialImmersion/Blueprint/Gamification/BP_Arrow_Rotation.StaticMesh` (`self.Arrow`)) false false)
      (`SceneComponent.SetVisibility` (`/Game/SpatialImmersion/Blueprint/Practice/Signs/BP_InfoSign_Handle.Exclmark` (`self.Sign`)) false false)
      (bind _returnvalue (`|CreateWidget` "/Game/SpatialImmersion/Blueprint/Practice/Signs/New_Task.New_Task_C"))
      (`WidgetComponent.SetWidget` (`/Game/SpatialImmersion/Blueprint/Practice/Signs/BP_InfoSign_Handle.Widget` (`self.Sign`)) _returnvalue))
    (else
      (`PrimitiveComponent.SetMaterial` (`self.StaticMesh`) 1 "/Game/SpatialImmersion/Material/Pattern/Museum/Pictures/Gleaners_Mat.Gleaners_Mat"))))

(fn `UserConstructionScript`)