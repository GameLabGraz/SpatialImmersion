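; Practice-area trigger for a VR teleport exercise that swaps guidance signs when the player arrives.
; A Timeline started at BeginPlay animates the guide Arrow by offsetting it from its starting world location.
; When a VRCharacterBase enters the Box, the Sign's parts appear and the SignTeleport's parts and Arrow hide.
; Leaving hides the Sign again but does not restore the teleport sign or Arrow.
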(event `self.ReceiveBeginPlay`
  (bind _output_get (set `self.Root Location` (`SceneComponent.K2_GetComponentLocation` (`self.Arrow`))))
  (bind (_direction _location) (`Timeline|Timeline_0`)
    (:`Update`
      (`SceneComponent.K2_SetWorldLocation` (`self.Arrow`) (+ _location _output_get) false false))))

(event `self.Box.OnComponentBeginOverlap`
  (params (OverlappedComponent :type "PrimitiveComponent Object Reference") (OtherActor :type "Actor Object Reference") (OtherComp :type "PrimitiveComponent Object Reference") (OtherBodyIndex :type Integer) (bFromSweep :type Boolean) (SweepResult :type "HitResult Structure (by ref)"))
  (cast `VRCharacterBase` OtherActor)
  (`SceneComponent.SetVisibility` (`/Game/SpatialImmersion/Blueprint/Practice/Signs/BP_InfoSign_Button.Widget` (`self.Sign`)) true false)
  (`SceneComponent.SetVisibility` (`/Game/SpatialImmersion/Blueprint/Practice/Signs/BP_InfoSign_Button.Exclmark` (`self.Sign`)) true false)
  (`SceneComponent.SetVisibility` (`/Game/SpatialImmersion/Blueprint/Practice/Signs/BP_InfoSign_Button.StaticMesh` (`self.Sign`)) true false)
  (`SceneComponent.SetVisibility` (`/Game/SpatialImmersion/Blueprint/Practice/Signs/BP_InfoSign_Teleport.StaticMesh` (`self.SignTeleport`)) false false)
  (`SceneComponent.SetVisibility` (`/Game/SpatialImmersion/Blueprint/Practice/Signs/BP_InfoSign_Teleport.Exclmark` (`self.SignTeleport`)) false false)
  (`SceneComponent.SetVisibility` (`/Game/SpatialImmersion/Blueprint/Practice/Signs/BP_InfoSign_Teleport.Widget` (`self.SignTeleport`)) false false)
  (`SceneComponent.SetVisibility` (`self.Arrow`) false false))

(event `self.Box.OnComponentEndOverlap`
  (params (OverlappedComponent :type "PrimitiveComponent Object Reference") (OtherActor :type "Actor Object Reference") (OtherComp :type "PrimitiveComponent Object Reference") (OtherBodyIndex :type Integer))
  (cast `VRCharacterBase` OtherActor)
  (`SceneComponent.SetVisibility` (`/Game/SpatialImmersion/Blueprint/Practice/Signs/BP_InfoSign_Button.Widget` (`self.Sign`)) false false)
  (`SceneComponent.SetVisibility` (`/Game/SpatialImmersion/Blueprint/Practice/Signs/BP_InfoSign_Button.Exclmark` (`self.Sign`)) false false)
  (`SceneComponent.SetVisibility` (`/Game/SpatialImmersion/Blueprint/Practice/Signs/BP_InfoSign_Button.StaticMesh` (`self.Sign`)) false false))

(fn `UserConstructionScript`)