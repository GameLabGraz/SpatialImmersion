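; BP_Slider_Practice is a slider practice station that recolors a statue as trigger boxes detect overlaps.
; Both boxes check TiggerBoxHandle's overlaps: Box turns the statue black, Box_Top turns it tan, and leaving restores white marble.
; The first successful Box_Top overlap, gated by the Spawn flag, advances the tutorial by revealing new torus, arrow and decal hints, hiding old ones and putting a New_Task widget on the sign.
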(event `self.ReceiveTick`
  (params (DeltaSeconds :type "Float (single-precision)")))

(event `self.Box.OnComponentBeginOverlap`
  (params (OverlappedComponent :type "PrimitiveComponent Object Reference") (OtherActor :type "Actor Object Reference") (OtherComp :type "PrimitiveComponent Object Reference") (OtherBodyIndex :type Integer) (bFromSweep :type Boolean) (SweepResult :type "HitResult Structure (by ref)"))
  (if (`PrimitiveComponent.IsOverlappingActor` (`self.TiggerBoxHandle`) OtherActor)
    (`PrimitiveComponent.SetMaterial` (`/Game/SpatialImmersion/Blueprint/Practice/Props/BP_Statue_Huge.StaticMesh` (`self.Statue`)) 0 "/Game/SpatialImmersion/Material/SmartArchViz/MI_BlackColor01.MI_BlackColor01")))

(event `self.Box.OnComponentEndOverlap`
  (params (OverlappedComponent :type "PrimitiveComponent Object Reference") (OtherActor :type "Actor Object Reference") (OtherComp :type "PrimitiveComponent Object Reference") (OtherBodyIndex :type Integer))
  (if (not (`PrimitiveComponent.IsOverlappingActor` (`self.TiggerBoxHandle`) OtherActor))
    (`PrimitiveComponent.SetMaterial` (`/Game/SpatialImmersion/Blueprint/Practice/Props/BP_Statue_Huge.StaticMesh` (`self.Statue`)) 0 "/Game/SpatialImmersion/Material/ArchViz/MI_Marble_White.MI_Marble_White")))

(event `self.Box_Top.OnComponentBeginOverlap`
  (params (OverlappedComponent :type "PrimitiveComponent Object Reference") (OtherActor :type "Actor Object Reference") (OtherComp :type "PrimitiveComponent Object Reference") (OtherBodyIndex :type Integer) (bFromSweep :type Boolean) (SweepResult :type "HitResult Structure (by ref)"))
  (if (`PrimitiveComponent.IsOverlappingActor` (`self.TiggerBoxHandle`) OtherActor)
    (`PrimitiveComponent.SetMaterial` (`/Game/SpatialImmersion/Blueprint/Practice/Props/BP_Statue_Huge.StaticMesh` (`self.Statue`)) 0 "/Game/SpatialImmersion/Material/ArchViz/MI_Marble_Tan.MI_Marble_Tan")
    (if (`self.Spawn`)
      (set `self.Spawn` false)
      (`SceneComponent.SetVisibility` (`/Game/SpatialImmersion/Blueprint/Practice/BP_Teleport_Torus_Door.StaticMesh` (`self.Torus_New01`)) true false)
      (`SceneComponent.SetVisibility` (`/Game/SpatialImmersion/Blueprint/Practice/BP_Teleport_Torus_Door.Arrow` (`self.Torus_New01`)) true false)
      (`SceneComponent.SetVisibility` (`/Game/SpatialImmersion/Blueprint/Practice/BP_Teleport_Torus_Door.Teleport_Torus` (`self.Torus_New01`)) true false)
      (`SceneComponent.SetVisibility` (`/Game/SpatialImmersion/Blueprint/Practice/BP_Teleport_Torus_Door.Arrow1` (`self.Torus_New01`)) true false)
      (`SceneComponent.SetVisibility` (`/Game/SpatialImmersion/Blueprint/Gamification/BP_Arrow_Hint.StaticMesh` (`self.Arrow_Hint`)) true false)
      (`SceneComponent.SetVisibility` (`DecalActor.Decal` (`self.Decal_New`)) true false)
      (`SceneComponent.SetVisibility` (`/Game/SpatialImmersion/Blueprint/Practice/BP_Teleport_Torus_Slider.StaticMesh` (`self.Torus_Old`)) false false)
      (`SceneComponent.SetVisibility` (`/Game/SpatialImmersion/Blueprint/Gamification/BP_Arrow_Small.StaticMesh` (`self.Arrow01`)) false false)
      (`SceneComponent.SetVisibility` (`/Game/SpatialImmersion/Blueprint/Gamification/BP_Arrow_Small.StaticMesh` (`self.Arrow02`)) false false)
      (`SceneComponent.SetVisibility` (`/Game/SpatialImmersion/Blueprint/Practice/Signs/BP_InfoSign_Slider.Exclmark` (`self.Sign`)) false false)
      (bind _returnvalue (`|CreateWidget` "/Game/SpatialImmersion/Blueprint/Practice/Signs/New_Task.New_Task_C"))
      (`WidgetComponent.SetWidget` (`/Game/SpatialImmersion/Blueprint/Practice/Signs/BP_InfoSign_Slider.Widget` (`self.Sign`)) _returnvalue))))

(event `self.Box_Top.OnComponentEndOverlap`
  (params (OverlappedComponent :type "PrimitiveComponent Object Reference") (OtherActor :type "Actor Object Reference") (OtherComp :type "PrimitiveComponent Object Reference") (OtherBodyIndex :type Integer))
  (if (not (`PrimitiveComponent.IsOverlappingActor` (`self.TiggerBoxHandle`) null))
    (`PrimitiveComponent.SetMaterial` (`/Game/SpatialImmersion/Blueprint/Practice/Props/BP_Statue_Huge.StaticMesh` (`self.Statue`)) 0 "/Game/SpatialImmersion/Material/ArchViz/MI_Marble_White.MI_Marble_White")))

(fn `UserConstructionScript`)