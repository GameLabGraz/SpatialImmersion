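; Exit teleporter actor that loads the VR_Breakroom level when a VR character enters its box trigger.
; The level change only happens while the Level flag on the referenced Column is set.
; On BeginPlay it hides the Arrow and StaticMesh without affecting their children, then a timeline moves the Arrow around its starting world location.
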(event `self.ReceiveBeginPlay`
  (`SceneComponent.SetVisibility` (`self.Arrow`) false false)
  (`SceneComponent.SetVisibility` (`self.StaticMesh`) false false)
  (bind _output_get (set `self.Root Location` (`SceneComponent.K2_GetComponentLocation` (`self.Arrow`))))
  (bind (_direction _location) (`Timeline|Timeline_0`)
    (:`Update`
      (`SceneComponent.K2_SetWorldLocation` (`self.Arrow`) (+ _location _output_get) false false))))

(event `self.Box.OnComponentBeginOverlap`
  (params (OverlappedComponent :type "PrimitiveComponent Object Reference") (OtherActor :type "Actor Object Reference") (OtherComp :type "PrimitiveComponent Object Reference") (OtherBodyIndex :type Integer) (bFromSweep :type Boolean) (SweepResult :type "HitResult Structure (by ref)"))
  (if (`/Game/SpatialImmersion/Blueprint/Practice/BP_Column.Level` (`self.Column`))
    (cast `VRCharacterBase` OtherActor)
    (`GameplayStatics.OpenLevel` "VR_Breakroom")))

(fn `UserConstructionScript`)