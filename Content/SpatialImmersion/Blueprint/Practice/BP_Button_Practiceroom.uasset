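; Physics-driven push button for the practice room that reveals the Vase and Lathe objects when triggered.
; On BeginPlay it joins the button's cube and cylinder with a Z-limited physics constraint and hides both props with collision and physics off.
; A Box overlap, confirmed by the cylinder overlapping the same actor, shows them, restores WorldStatic blocking and WorldDynamic overlap, and starts physics simulation.
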(event `self.ReceiveBeginPlay`
  (bind _staticmeshcomponent (`PickupActor.StaticMeshComponent` (`self.Vase`)))
  (`PhysicsConstraintComponent.SetConstrainedComponents` (`self.PhysicsConstraint`) (`self.Button_Mesh_Cube`) "None" (`self.Button_Mesh_Cylinder`) "None")
  (`PhysicsConstraintComponent.SetLinearZLimit` (`self.PhysicsConstraint`) "LCM_Limited" 4.0)
  (`SceneComponent.SetVisibility` _staticmeshcomponent false false)
  (`SceneComponent.SetVisibility` (`PickupActor.StaticMeshComponent` (`self.Lathe`)) false false)
  (`PrimitiveComponent.SetCollisionResponseToAllChannels` _staticmeshcomponent "ECR_Ignore")
  (`PrimitiveComponent.SetCollisionResponseToAllChannels` (`PickupActor.StaticMeshComponent` (`self.Lathe`)) "ECR_Ignore")
  (`PrimitiveComponent.SetSimulatePhysics` _staticmeshcomponent false)
  (`PrimitiveComponent.SetSimulatePhysics` (`PickupActor.StaticMeshComponent` (`self.Lathe`)) false))

(event `self.Box.OnComponentBeginOverlap`
  (params (OverlappedComponent :type "PrimitiveComponent Object Reference") (OtherActor :type "Actor Object Reference") (OtherComp :type "PrimitiveComponent Object Reference") (OtherBodyIndex :type Integer) (bFromSweep :type Boolean) (SweepResult :type "HitResult Structure (by ref)"))
  (bind _staticmeshcomponent (`PickupActor.StaticMeshComponent` (`self.Vase`)))
  (if (`PrimitiveComponent.IsOverlappingActor` (`self.Button_Mesh_Cylinder`) OtherActor)
    (`SceneComponent.SetVisibility` _staticmeshcomponent true false)
    (`SceneComponent.SetVisibility` (`PickupActor.StaticMeshComponent` (`self.Lathe`)) true false)
    (`PrimitiveComponent.SetCollisionResponseToChannel` _staticmeshcomponent "ECC_WorldStatic" "ECR_Block")
    (`PrimitiveComponent.SetCollisionResponseToChannel` (`PickupActor.StaticMeshComponent` (`self.Lathe`)) "ECC_WorldStatic" "ECR_Block")
    (`PrimitiveComponent.SetCollisionResponseToChannel` _staticmeshcomponent "ECC_WorldDynamic" "ECR_Overlap")
    (`PrimitiveComponent.SetCollisionResponseToChannel` (`PickupActor.StaticMeshComponent` (`self.Lathe`)) "ECC_WorldDynamic" "ECR_Overlap")
    (`PrimitiveComponent.SetSimulatePhysics` (`PickupActor.StaticMeshComponent` (`self.Lathe`)) true)
    (`PrimitiveComponent.SetSimulatePhysics` _staticmeshcomponent true)))

(fn `UserConstructionScript`)