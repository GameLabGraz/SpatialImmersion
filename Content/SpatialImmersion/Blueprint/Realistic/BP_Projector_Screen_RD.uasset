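; BP_Projector_Screen_RD is a projector screen actor with four realistic star components that appear as objects register on a linked Shelf.
; All stars are hidden on BeginPlay.
; Every Tick, four functions poll the Shelf's overlap flags and each shows its matching star.
; Stars are never hidden again during play, so each reveal stays once triggered.
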(event `self.ReceiveBeginPlay`
  (`self.Set Stars Invisible`))

(event `self.ReceiveTick`
  (params (DeltaSeconds :type "Float (single-precision)"))
  (`self.Set Star Visible`)
  (`self.Set Star1 Visible`)
  (`self.Set Star2 Visible`)
  (`self.Set Star3 Visible`))

(fn `Set Star Visible`
  (if (`/Game/SpatialImmersion/Blueprint/UMG/Realisitc/Dark/BP_Shelf_Long_Realist_Dark.OverlapObject01` (`self.Shelf`))
    (`SceneComponent.SetVisibility` (`self.Star_Realistic`) true false)))

(fn `Set Star1 Visible`
  (if (`/Game/SpatialImmersion/Blueprint/UMG/Realisitc/Dark/BP_Shelf_Long_Realist_Dark.OverlapObject02` (`self.Shelf`))
    (`SceneComponent.SetVisibility` (`self.Star_Realistic1`) true false)))

(fn `Set Star2 Visible`
  (if (`/Game/SpatialImmersion/Blueprint/UMG/Realisitc/Dark/BP_Shelf_Long_Realist_Dark.OverlapObject03` (`self.Shelf`))
    (`SceneComponent.SetVisibility` (`self.Star_Realistic2`) true false)))

(fn `Set Star3 Visible`
  (if (`/Game/SpatialImmersion/Blueprint/UMG/Realisitc/Dark/BP_Shelf_Long_Realist_Dark.OverlapObject04` (`self.Shelf`))
    (`SceneComponent.SetVisibility` (`self.Star_Realistic3`) true false)))

(fn `Set Stars Invisible`
  (`SceneComponent.SetVisibility` (`self.Star_Realistic`) false false)
  (`SceneComponent.SetVisibility` (`self.Star_Realistic1`) false false)
  (`SceneComponent.SetVisibility` (`self.Star_Realistic2`) false false)
  (`SceneComponent.SetVisibility` (`self.Star_Realistic3`) false false))

(fn `UserConstructionScript`)