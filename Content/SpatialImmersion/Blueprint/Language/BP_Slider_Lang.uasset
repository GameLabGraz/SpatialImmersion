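; BP_Slider_Lang is a slider actor that switches the game's language between English and German.
; Overlap events on the English and German boxes check whether the handle's trigger box overlaps the same actor, then set the current culture.
; The handle mesh material shows the selection, dark blue for English and matte red for German.
; On end overlap it turns black if the trigger box no longer overlaps that actor.
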(event `self.ReceiveBeginPlay`)

(event `self.Box_English.OnComponentBeginOverlap`
  (params (OverlappedComponent :type "PrimitiveComponent Object Reference") (OtherActor :type "Actor Object Reference") (OtherComp :type "PrimitiveComponent Object Reference") (OtherBodyIndex :type Integer) (bFromSweep :type Boolean) (SweepResult :type "HitResult Structure (by ref)"))
  (if (`PrimitiveComponent.IsOverlappingActor` (`self.TiggerBoxHandle`) OtherActor)
    (`KismetInternationalizationLibrary.SetCurrentCulture` "en")
    (`PrimitiveComponent.SetMaterial` (`self.HandleStaticMesh`) 0 "/Game/Cartoon_Furniture/Materials/Colours/_Blue_Dark_._Blue_Dark_")))

(event `self.Box_English.OnComponentEndOverlap`
  (params (OverlappedComponent :type "PrimitiveComponent Object Reference") (OtherActor :type "Actor Object Reference") (OtherComp :type "PrimitiveComponent Object Reference") (OtherBodyIndex :type Integer))
  (if (not (`PrimitiveComponent.IsOverlappingActor` (`self.TiggerBoxHandle`) OtherActor))
    (`PrimitiveComponent.SetMaterial` (`self.HandleStaticMesh`) 0 "/Game/Cartoon_Furniture/Materials/Colours/_Black_2_._Black_2_")))

(event `self.Box_German.OnComponentBeginOverlap`
  (params (OverlappedComponent :type "PrimitiveComponent Object Reference") (OtherActor :type "Actor Object Reference") (OtherComp :type "PrimitiveComponent Object Reference") (OtherBodyIndex :type Integer) (bFromSweep :type Boolean) (SweepResult :type "HitResult Structure (by ref)"))
  (if (`PrimitiveComponent.IsOverlappingActor` (`self.TiggerBoxHandle`) OtherActor)
    (`KismetInternationalizationLibrary.SetCurrentCulture` "de")
    (`PrimitiveComponent.SetMaterial` (`self.HandleStaticMesh`) 0 "/Game/Cartoon_Furniture/Materials/Colours/_Red_Matt_._Red_Matt_")))

(event `self.Box_German.OnComponentEndOverlap`
  (params (OverlappedComponent :type "PrimitiveComponent Object Reference") (OtherActor :type "Actor Object Reference") (OtherComp :type "PrimitiveComponent Object Reference") (OtherBodyIndex :type Integer))
  (if (not (`PrimitiveComponent.IsOverlappingActor` (`self.TiggerBoxHandle`) OtherActor))
    (`PrimitiveComponent.SetMaterial` (`self.HandleStaticMesh`) 0 "/Game/Cartoon_Furniture/Materials/Colours/_Black_2_._Black_2_")))

(fn `UserConstructionScript`)