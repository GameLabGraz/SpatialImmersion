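; Frame_01_Big is an actor that reveals a Robot once two referenced handles, left and middle, are both rotated past a threshold.
; BeginPlay hides the Robot's mesh, disables its physics and sets it to ignore world static and dynamic collision.
; Tick polls both handle rotations, then destroys the Arrow actor, shows the Robot and enables its collision and physics, using the Spawn flag to fire only once.
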(event `self.ReceiveBeginPlay`
  (bind _staticmeshcomponent (`PickupActor.StaticMeshComponent` (`self.Robot`)))
  (`SceneComponent.SetVisibility` _staticmeshcomponent false false)
  (`PrimitiveComponent.SetCollisionResponseToChannel` _staticmeshcomponent "ECC_WorldStatic" "ECR_Ignore")
  (`PrimitiveComponent.SetCollisionResponseToChannel` _staticmeshcomponent "ECC_WorldDynamic" "ECR_Ignore")
  (`PrimitiveComponent.SetSimulatePhysics` _staticmeshcomponent false))

(event `self.ReceiveTick`
  (params (DeltaSeconds :type "Float (single-precision)"))
  (bind _staticmeshcomponent (`PickupActor.StaticMeshComponent` (`self.Robot`)))
  (if (and (> (`CircularDriveActor.CurrentRotation` (`self.Handle Left`)) 80.0) (> (`CircularDriveActor.CurrentRotation` (`self.Handle Middle`)) 80.0) (`self.Spawn`))
    (`self.K2_DestroyActor` (`self.Arrow`))
    (`SceneComponent.SetVisibility` _staticmeshcomponent true false)
    (`PrimitiveComponent.SetCollisionResponseToChannel` _staticmeshcomponent "ECC_WorldStatic" "ECR_Block")
    (`PrimitiveComponent.SetCollisionResponseToChannel` _staticmeshcomponent "ECC_WorldDynamic" "ECR_Overlap")
    (`PrimitiveComponent.SetSimulatePhysics` _staticmeshcomponent true)
    (set `self.Spawn` false)))

(fn `UserConstructionScript`)