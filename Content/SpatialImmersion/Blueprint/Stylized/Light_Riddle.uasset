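; Light riddle Blueprint that drives a spotlight, hidden at start, from the rotation of a referenced Handle.
; While the handle's rotation exceeds 95, Tick feeds a one-second Delay, so the color advances about once per second.
; ChangeLightColor shows the light and uses a counter to cycle green, blue, red and white.
; Nothing hides the light again once it is shown.
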(event `self.ReceiveBeginPlay`
  (`SceneComponent.SetVisibility` (`self.SpotLight`) false false))

(event `self.ReceiveTick`
  (params (DeltaSeconds :type "Float (single-precision)"))
  (if (> (`CircularDriveActor.CurrentRotation` (`self.Handle`)) 95.0)
    (`KismetSystemLibrary.Delay` 1.0)
    (`self.Change Light color`)))

(fn `Change Light color`
  (`SceneComponent.SetVisibility` (`self.SpotLight`) true false)
  (if (== (`self.Counter`) 0)
    (`LightComponent.SetLightColor` (`self.SpotLight`) (struct :`G` 0.385417 :`B` 0.015203 :`A` 1.0) true)
    (set `self.Counter` 1)
    (elif (== (`self.Counter`) 1)
      (`LightComponent.SetLightColor` (`self.SpotLight`) (struct :`R` 0.002372 :`G` 0.009213 :`B` 0.479167 :`A` 1.0) true)
      (set `self.Counter` 2)
      (elif (== (`self.Counter`) 2)
        (`LightComponent.SetLightColor` (`self.SpotLight`) (struct :`R` 0.328125 :`G` 0.003133 :`A` 1.0) true)
        (set `self.Counter` 3)
        (else
          (`LightComponent.SetLightColor` (`self.SpotLight`) (struct :`R` 1.0 :`G` 0.989583 :`B` 0.989583 :`A` 1.0) true)
          (set `self.Counter` 0))))))

(fn `UserConstructionScript`)